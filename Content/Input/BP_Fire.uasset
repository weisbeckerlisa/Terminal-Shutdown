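; BP_Fire is an extinguishable Niagara fire that reports to a MiniGameController and starts hidden.
; ApplyFireScale activates and shows it with a given scale value.
; While active, ApplyExtinguish shrinks that value and the effect by time, strength and ExtinguishRate, hiding it and notifying the controller at zero, without clearing IsActive.
; A collision sphere tracks PlayerInRange from BP_FireExtinguisher overlaps, which ApplyExtinguish does not check.
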(event OnComponentBeginOverlap(SphereCollision)
  (params (OverlappedComponent :type Primitive%20Component%20Object%20Reference) (OtherActor :type Actor%20Object%20Reference) (OtherComp :type Primitive%20Component%20Object%20Reference) (OtherBodyIndex :type Integer) (bFromSweep :type Boolean) (SweepResult :type Hit%20Result%20Structure%20%28by%20ref%29))
  (Utilities|Casting|CastToBP_FireExtinguisher OtherActor)
  (Variables|Default|SetbPlayerInRange true)
  (Development|PrintString "In range"))

(event OnComponentEndOverlap(SphereCollision)
  (params (OverlappedComponent :type Primitive%20Component%20Object%20Reference) (OtherActor :type Actor%20Object%20Reference) (OtherComp :type Primitive%20Component%20Object%20Reference) (OtherBodyIndex :type Integer))
  (Utilities|Casting|CastToBP_FireExtinguisher OtherActor)
  (Variables|Default|SetbPlayerInRange false)
  (Development|PrintString "Out of range"))

(event EventBeginPlay
  (bind _output_get (Variables|Default|SetbIsActive false))
  (Rendering|SetVisibility (Variables|NiagaraActor|GetNiagaraComponent) _output_get true)
  (bind _output_get_2 (Variables|Default|SetFireScale 0.0))
  (Development|PrintString (Utilities|String|ToString(Float) _output_get_2)))

(event EventTick
  (params (DeltaSeconds :type Float%20%28single-precision%29)))

(fn ConstructionScript)

(fn ApplyExtinguish
  (params (DeltaSeconds :type Float%20%28double-precision%29) (Strength :type Float%20%28double-precision%29))
  (bind _niagaracomponent (Variables|NiagaraActor|GetNiagaraComponent))
  (if (Variables|Default|GetbIsActive)
    (bind _output_get (Variables|Default|SetFireScale (Math|Float|Max(Float) 0.0 (- (Variables|Default|GetFireScale) (* DeltaSeconds Strength (Variables|Default|GetExtinguishRate))))))
    (Transformation|SetWorldScale3D _niagaracomponent (Math|Vector|MakeVector _output_get _output_get _output_get))
    (if (<= (Variables|Default|GetFireScale) 0.0)
      (Rendering|SetVisibility _niagaracomponent false true)
      (Default|NotifyFireState (Variables|Default|GetMiniGameController)))))

(fn ApplyFireScale
  (params (FireScale :type Float%20%28double-precision%29))
  (bind _output_get (Variables|Default|SetbIsActive true))
  (Rendering|SetVisibility (Variables|NiagaraActor|GetNiagaraComponent) _output_get true)
  (bind _output_get_2 (Variables|Default|SetFireScale FireScale))
  (Development|PrintString (Utilities|String|ToString(Float) _output_get_2)))