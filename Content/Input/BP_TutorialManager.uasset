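; Tutorial manager actor that plays the intro Level Sequence when the level begins, then moves the scene out of its alarm state.
; BeginPlay creates a sequence player and binds its finished event to NextSteps.
; NextSteps fades out the referenced alarm's sound, waits briefly, then hides the alarm's two spotlights and shows two other referenced lights.
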(event Custom|Next%20steps
  (bind _alarmref (Variables|Default|GetAlarmRef))
  (Audio|Components|Audio|FadeOut (Variables|/Game/Input/BP_Alarm.BP_Alarm_C|GetAlarmSound _alarmref) 3.0 0.0 "Linear" :!class /Script/Engine.AudioComponent)
  (Utilities|FlowControl|Delay 3.0)
  (Rendering|SetVisibility (Variables|/Game/Input/BP_Alarm.BP_Alarm_C|GetSpotLight _alarmref) false false)
  (Rendering|SetVisibility (Variables|/Game/Input/BP_Alarm.BP_Alarm_C|GetSpotLight1 _alarmref) false false)
  (Rendering|SetVisibility (Variables|/Script/Engine.Light|GetLightComponent (Variables|Default|GetLight1Ref)) true false)
  (Rendering|SetVisibility (Variables|/Script/Engine.Light|GetLightComponent (Variables|Default|GetLight2Ref)) true false))

(event EventBeginPlay
  (bind _returnvalue (Sequencer|Player|CreateLevelSequencePlayer (Variables|Default|GetIntroSequence)))
  (bind _output_get (Variables|Default|SetLSPlayer _returnvalue))
  (EventDispatchers|BindEventtoOnFinished _output_get (delegate Custom|Next%20steps))
  (Sequencer|Player|Play _output_get :!class /Script/MovieScene.MovieSceneSequencePlayer))

(event Collision|EventActorBeginOverlap
  (params (OtherActor :type Actor%20Object%20Reference)))

(event EventTick
  (params (DeltaSeconds :type Float%20%28single-precision%29)))

(fn ConstructionScript)