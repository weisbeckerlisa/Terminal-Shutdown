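; Mini-game runner actor that drives the FireOut and LightsOff mini-games through the event run subsystem.
; It tracks the active gameplay tag from subsystem start events and relays end logs through OnMiniGameCompleted.
; For FireOut, it scales up the fire, then applies extinguishing each Tick while click is held and the player is in range.
; Notify functions report success when the fire state is notified or both switches are off.
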(event Custom|HandleMiniGameStarted
  (params (Context :type Mini%20Game%20Context%20Structure%20%28by%20ref%29))
  (bind _output_get (Variables|Default|SetCurrentMiniGame (Variables|/Script/TerminalShutdown.MiniGameDefinition|GetMiniGameTag (.Definition (Utilities|Struct|BreakMiniGameContext Context)))))
  (if (GameplayTags|MatchesTag _output_get "(TagName=\"MiniGame.FireOut\")" true)
    (Development|PrintString "Quick, extinguish the fire !")
    (Default|ApplyFireScale (Variables|Default|GetFireTarget) 2.0)))

(event Custom|HandleMiniGameEnded
  (params (Result :type EMiniGameResult%20Enum :default "Success") (Logs :type Array%20of%20Texts))
  (Default|CallOnMiniGameCompleted Logs))

(event Input|EnhancedActionEvents|EnhancedInputActionIA_Click
  (params (ActionValue :type Boolean) (ElapsedSeconds :type Float%20%28double-precision%29) (TriggeredSeconds :type Float%20%28double-precision%29) (InputAction :type Input%20Action%20Object%20Reference :default "/Game/Input/Actions/IA_Click.IA_Click"))
  (:Started
    (Variables|Default|SetbSpraying true))
  (:Canceled
    (Variables|Default|SetbSpraying false))
  (:Completed
    (Variables|Default|SetbSpraying false)))

(event EventBeginPlay
  (bind _output_get (Variables|Default|SetSubsystemRef (Subsystems|GetEventRunSubsystem)))
  (EventDispatchers|BindEventtoOnMiniGameStarted _output_get (delegate Custom|HandleMiniGameStarted))
  (EventDispatchers|BindEventtoOnMiniGameEnded _output_get (delegate Custom|HandleMiniGameEnded))
  (Input|EnableInput (Game|GetPlayerController 0)))

(event Collision|EventActorBeginOverlap
  (params (OtherActor :type Actor%20Object%20Reference)))

(event EventTick
  (params (DeltaSeconds :type Float%20%28single-precision%29))
  (bind _firetarget (Variables|Default|GetFireTarget))
  (if (GameplayTags|MatchesTag (Variables|Default|GetCurrentMiniGame) "(TagName=\"MiniGame.FireOut\")" true)
    (Utilities|IsValid (Variables|Default|GetFireExtinguisher)
      (:Is%20Valid
        (Utilities|IsValid _firetarget
          (:Is%20Valid
            (if (Variables|Default|GetbSpraying)
              (if (Variables|/Game/Input/BP_Fire.BP_Fire_C|GetbPlayerInRange _firetarget)
                (Default|ApplyExtinguish _firetarget DeltaSeconds 1.0)))))))))

(fn ConstructionScript)

(fn NotifySwitchState
  (params (Index :type Integer) (bIsOff :type Boolean))
  (switch int Index
    (:0
      (bind _output_get (Variables|Default|SetbOff0 bIsOff)))
    (:1
      (bind _output_get_2 (Variables|Default|SetbOff1 bIsOff))))
  (if (and _output_get _output_get_2)
    (if (GameplayTags|MatchesTag (Variables|Default|GetCurrentMiniGame) "(TagName=\"MiniGame.LightsOff\")" true)
      (Class|EventRunSubsystem|CompleteMiniGame (Variables|Default|GetSubsystemRef) "Success"))))

(fn NotifyFireState
  (if (GameplayTags|MatchesTag (Variables|Default|GetCurrentMiniGame) "(TagName=\"MiniGame.FireOut\")" true)
    (Class|EventRunSubsystem|CompleteMiniGame (Variables|Default|GetSubsystemRef) "Success")))