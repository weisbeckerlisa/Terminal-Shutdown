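; BP_Button is an interactable toggle button that switches a tagged ship module on or off.
; On BeginPlay it creates a dynamic material instance on its mesh with the emissive glow off.
; Interact flips IsOn, passes it with ModuleTag to the player pawn's ShipStateComponent, and sets EmissiveStrength to match.
; The toggle only happens when that component is found on the pawn.
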(event EventBeginPlay
  (bind _returnvalue (Rendering|Material|CreateDynamicMaterialInstance (Variables|Debug|GetStaticMeshComponent) 0 0 "None" :!class /Script/Engine.PrimitiveComponent))
  (bind _output_get (Variables|Default|SetButtonMID _returnvalue))
  (Rendering|Material|SetScalarParameterValue _output_get "EmissiveStrength" 0.0 :!class /Script/Engine.MaterialInstanceDynamic))

(event Collision|EventActorBeginOverlap
  (params (OtherActor :type Actor%20Object%20Reference)))

(event EventTick
  (params (DeltaSeconds :type Float%20%28single-precision%29)))

(event EventInteract
  (bind _returnvalue (Game|Player|GetPlayerPawn 0))
  (bind _returnvalue_2 (Actor|GetComponentbyClass _returnvalue "/Script/TerminalShutdown.ShipStateComponent"))
  (Utilities|IsValid _returnvalue_2
    (:Is%20Valid
      (bind _output_get (Variables|Default|SetbIsOn (not (Variables|Default|GetbIsOn))))
      (Class|ShipStateComponent|SetModuleEnabled _returnvalue_2 (Variables|Default|GetModuleTag) _output_get)
      (if (Variables|Default|GetbIsOn)
        (Rendering|Material|SetScalarParameterValue (stale EventBeginPlay _output_get) "EmissiveStrength" 1.0 :!class /Script/Engine.MaterialInstanceDynamic)
        (else
          (Rendering|Material|SetScalarParameterValue (stale EventBeginPlay _output_get) "EmissiveStrength" 0.0 :!class /Script/Engine.MaterialInstanceDynamic))))))

(fn ConstructionScript)