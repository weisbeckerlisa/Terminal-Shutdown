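; Signal-matching minigame terminal where the player tunes frequency, amplitude and phase of a wave to match a random target.
; StartMG rolls the target, draws both waves through a dynamic material on the screen plane and initializes the widget display.
; Three button colliders decrease, cycle or increase the selected parameter, refreshing material and widget.
; Each adjustment compares sampled sine curves by mean absolute error, notifying MiniGameManager once below the win threshold.
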(event Custom|StartMG
  (CallFunction|InitTargetValues)
  (bind _returnvalue (Rendering|Material|CreateDynamicMaterialInstance "/Game/Materials/M_UI_SignalPlot.M_UI_SignalPlot" "MI_UI_SignalPlot" "None" :!class /Script/Engine.KismetMaterialLibrary))
  (bind _output_get (Variables|Default|SetMI_Signal _returnvalue))
  (CallFunction|RefreshSignalMat)
  (Rendering|Material|SetMaterial (Variables|Default|GetScreenPlane) 0 _output_get)
  (bind _aswbp_signal_display (Utilities|Casting|CastToWBP_SignalDisplay (UserInterface|GetUserWidgetObject (Variables|Default|GetWidget))))
  (Default|InitDisplay _aswbp_signal_display (Variables|Default|GetPlayerFrequency) (Variables|Default|GetPlayerAmplitude) (Variables|Default|GetPlayerPhase)))

(event EventBeginPlay)

(event Collision|EventActorBeginOverlap
  (params (OtherActor :type Actor%20Object%20Reference)))

(event EventTick
  (params (DeltaSeconds :type Float%20%28single-precision%29)))

(event EventInteract
  (params (Hit :type Hit%20Result%20Structure))
  (bind _hitcomponent (Collision|BreakHitResult Hit))
  (if (== _hitcomponent (Variables|Default|GetButton_Left_Collision))
    (CallFunction|DecreaseCurrentParameter)
    (CallFunction|CheckCompletion)
    (elif (== _hitcomponent (Variables|Default|GetButton_Middle_Collision))
      (CallFunction|CycleSelectedParameter)
      (elif (== _hitcomponent (Variables|Default|GetButton_Right_Collision))
        (CallFunction|IncreaseCurrentParameter)
        (CallFunction|CheckCompletion)))))

(fn ConstructionScript)

(fn RefreshSignalMat
  (bind _mi_signal (Variables|Default|GetMI_Signal))
  (Rendering|Material|SetScalarParameterValue _mi_signal "FrequencyTarget" (Variables|Default|GetTargetFrequency) :!class /Script/Engine.MaterialInstanceDynamic)
  (Rendering|Material|SetScalarParameterValue _mi_signal "AmplitudeTarget" (Variables|Default|GetTargetAmplitude) :!class /Script/Engine.MaterialInstanceDynamic)
  (Rendering|Material|SetScalarParameterValue _mi_signal "PhaseTarget" (Variables|Default|GetTargetPhase) :!class /Script/Engine.MaterialInstanceDynamic)
  (Rendering|Material|SetScalarParameterValue _mi_signal "Frequency" (Variables|Default|GetPlayerFrequency) :!class /Script/Engine.MaterialInstanceDynamic)
  (Rendering|Material|SetScalarParameterValue _mi_signal "Amplitude" (Variables|Default|GetPlayerAmplitude) :!class /Script/Engine.MaterialInstanceDynamic)
  (Rendering|Material|SetScalarParameterValue _mi_signal "Phase" (Variables|Default|GetPlayerPhase) :!class /Script/Engine.MaterialInstanceDynamic))

(fn CycleSelectedParameter
  (switch Utilities|FlowControl|Switch|SwitchonESignalParameter (Variables|Default|GetCurrentParameter)
    (:NewEnumerator0
      (Variables|Default|SetCurrentParameter "NewEnumerator1"))
    (:NewEnumerator1
      (Variables|Default|SetCurrentParameter "NewEnumerator2"))
    (:NewEnumerator2
      (Variables|Default|SetCurrentParameter "NewEnumerator0")))
  (CallFunction|RefreshParameterDisplay))

(fn RefreshParameterDisplay
  (bind _currentparameter (Variables|Default|GetCurrentParameter))
  (bind _aswbp_signal_display (Utilities|Casting|CastToWBP_SignalDisplay (UserInterface|GetUserWidgetObject (Variables|Default|GetWidget))))
  (switch Utilities|FlowControl|Switch|SwitchonESignalParameter _currentparameter
    (:NewEnumerator0
      (Default|RefreshDisplay _aswbp_signal_display _currentparameter (Variables|Default|GetPlayerFrequency)))
    (:NewEnumerator1
      (Default|RefreshDisplay _aswbp_signal_display _currentparameter (Variables|Default|GetPlayerAmplitude)))
    (:NewEnumerator2
      (Default|RefreshDisplay _aswbp_signal_display _currentparameter (Variables|Default|GetPlayerPhase)))))

(fn DecreaseCurrentParameter
  (switch Utilities|FlowControl|Switch|SwitchonESignalParameter (Variables|Default|GetCurrentParameter)
    (:NewEnumerator0
      (Variables|Default|SetPlayerFrequency (Math|Float|Clamp(Float) (- (Variables|Default|GetPlayerFrequency) (Variables|Default|GetFrequencyStep)) (Variables|Default|GetMinFrequency) (Variables|Default|GetMaxFrequency))))
    (:NewEnumerator1
      (Variables|Default|SetPlayerAmplitude (Math|Float|Clamp(Float) (- (Variables|Default|GetPlayerAmplitude) (Variables|Default|GetAmplitudeStep)) (Variables|Default|GetMinAmplitude) (Variables|Default|GetMaxAmplitude))))
    (:NewEnumerator2
      (Variables|Default|SetPlayerPhase (Math|Float|Clamp(Float) (- (Variables|Default|GetPlayerPhase) (Variables|Default|GetPhaseStep)) (Variables|Default|GetMinPhase) (Variables|Default|GetMaxPhase)))))
  (CallFunction|RefreshSignalMat)
  (CallFunction|RefreshParameterDisplay))

(fn IncreaseCurrentParameter
  (switch Utilities|FlowControl|Switch|SwitchonESignalParameter (Variables|Default|GetCurrentParameter)
    (:NewEnumerator0
      (Variables|Default|SetPlayerFrequency (Math|Float|Clamp(Float) (+ (Variables|Default|GetPlayerFrequency) (Variables|Default|GetFrequencyStep)) (Variables|Default|GetMinFrequency) (Variables|Default|GetMaxFrequency))))
    (:NewEnumerator1
      (Variables|Default|SetPlayerAmplitude (Math|Float|Clamp(Float) (+ (Variables|Default|GetPlayerAmplitude) (Variables|Default|GetAmplitudeStep)) (Variables|Default|GetMinAmplitude) (Variables|Default|GetMaxAmplitude))))
    (:NewEnumerator2
      (Variables|Default|SetPlayerPhase (Math|Float|Clamp(Float) (+ (Variables|Default|GetPlayerPhase) (Variables|Default|GetPhaseStep)) (Variables|Default|GetMinPhase) (Variables|Default|GetMaxPhase)))))
  (CallFunction|RefreshSignalMat)
  (CallFunction|RefreshParameterDisplay))

(fn InitTargetValues
  (Variables|Default|SetTargetFrequency (Math|Random|RandomFloatinRange (Variables|Default|GetMinFrequency) (Variables|Default|GetMaxFrequency)))
  (Variables|Default|SetTargetAmplitude (Math|Random|RandomFloatinRange (Variables|Default|GetMinAmplitude) (Variables|Default|GetMaxAmplitude)))
  (Variables|Default|SetTargetPhase (Math|Random|RandomFloatinRange (Variables|Default|GetMinPhase) (Variables|Default|GetMaxPhase))))

(fn CheckCompletion
  (if (not (Variables|Default|GetbIsSolved))
    (bind _error (CallFunction|ComputeSignalError))
    (bind _output_get (Variables|Default|SetCurrentError _error))
    (if (< _output_get (Variables|Default|GetWinThreshold))
      (Variables|Default|SetbIsSolved true)
      (Development|PrintString "Success")
      (Default|NotifySignalMatched (Variables|Default|GetMiniGameManager)))))

(fn EvaluateSignalatX
  (params (X :type Float%20%28double-precision%29) (Frequency :type Float%20%28double-precision%29) (Amplitude :type Float%20%28double-precision%29) (Phase :type Float%20%28double-precision%29))
  (return (* (Math|Trig|Sin(Radians) (+ (* (* X Frequency) 3.14159) Phase)) Amplitude)))

(fn ComputeSignalError
  (bind _samplecount (LocalVariables|GetSampleCount))
  (bind _returnvalue (- _samplecount 1))
  (LocalVariables|SetTotalError 0.0)
  (for _index (range 0 _returnvalue)
    (bind _output_get (LocalVariables|SetAlpha (/ _index (Math|Conversions|ToFloat(Integer) _returnvalue))))
    (bind _output_get_2 (LocalVariables|SetX (Math|Float|Lerp -1.0 1.0 _output_get)))
    (bind _y (CallFunction|EvaluateSignalatX _output_get_2 (Variables|Default|GetTargetFrequency) (Variables|Default|GetTargetAmplitude) (Variables|Default|GetTargetPhase)))
    (bind _y_2 (CallFunction|EvaluateSignalatX _output_get_2 (Variables|Default|GetPlayerFrequency) (Variables|Default|GetPlayerAmplitude) (Variables|Default|GetPlayerPhase)))
    (bind _output_get_3 (LocalVariables|SetDiff (Math|Float|Absolute(Float) (- _y _y_2))))
    (LocalVariables|SetTotalError (+ (LocalVariables|GetTotalError) _output_get_3)))
  (return (/ (LocalVariables|GetTotalError) _samplecount)))