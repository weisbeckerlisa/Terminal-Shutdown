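; BP_TutorialManager runs the game's opening: an optional alarm intro sequence, then a voice-over tutorial for the terminal and shelf, or an immediate run start.
; Lines play sequentially from a queue, with each audio finish incrementing a counter that drives hard-coded marker, widget highlight and vitals UI cues.
; Terminal and shelf stages begin on overlap notifications, gated by current step and idle voice-over, which is not rechecked when audio ends.
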(event Custom|Next%20steps
  (bind _terminalref (Variables|Default|GetTerminalRef))
  (Rendering|SetActorHiddenInGame (Game|GetPlayerCharacter 0) false)
  (bind _aswbp_planet_choices (Utilities|Casting|CastToWBP_PlanetChoices (UserInterface|GetUserWidgetObject (Variables|/Game/Blueprints/BP_Terminal.BP_Terminal_C|GetPlanetChoices_WidgetScreen _terminalref))))
  (bind _aswbp_planet_choices_overlay (Utilities|Casting|CastToWBP_PlanetChoices_Overlay (UserInterface|GetUserWidgetObject (Variables|/Game/Blueprints/BP_Terminal.BP_Terminal_C|GetPlanetChoices_Overlay _terminalref))))
  (Variables|Default|SetWBP_PlanetChoices_Overlay _aswbp_planet_choices_overlay)
  (bind _aswbp_planet_details_a_overlay (Utilities|Casting|CastToWBP_PlanetDetails_A_Overlay (UserInterface|GetUserWidgetObject (Variables|/Game/Blueprints/BP_Terminal.BP_Terminal_C|GetPlanetDetails_A_Overlay _terminalref))))
  (Variables|Default|SetWBP_PlanetDetails_A_Overlay _aswbp_planet_details_a_overlay)
  (bind _aswbp_planet_details_b_overlay (Utilities|Casting|CastToWBP_PlanetDetails_B_Overlay (UserInterface|GetUserWidgetObject (Variables|/Game/Blueprints/BP_Terminal.BP_Terminal_C|GetPlanetDetails_B_Overlay _terminalref))))
  (Variables|Default|SetWBP_PlanetDetails_B_Overlay _aswbp_planet_details_b_overlay)
  (bind _aswbp_modules_overlay (Utilities|Casting|CastToWBP_Modules_Overlay (UserInterface|GetUserWidgetObject (Variables|/Game/Blueprints/BP_Terminal.BP_Terminal_C|GetModules_Overlay _terminalref))))
  (Variables|Default|SetWBP_Modules_Overlay _aswbp_modules_overlay)
  (Utilities|FlowControl|Delay 3.0)
  (Default|StartRun _aswbp_planet_choices)
  (Utilities|FlowControl|Delay 4.0)
  (CallFunction|QueueVO "/Game/Audio/VoiceLines/Wav/WakeUp11_Tutorial.WakeUp11_Tutorial")
  (CallFunction|QueueVO "/Game/Audio/VoiceLines/Wav/WakeUp12.WakeUp12")
  (Math|Integer|IncrementInt (Variables|Default|GetCurrentStep)))

(event Custom|OnVOFinished
  (Utilities|FlowControl|Delay 1.0)
  (Math|Integer|IncrementInt (Variables|Default|GetVO_Counter)
    (:%20%20
      (CallFunction|CheckforHint)
      (CallFunction|PlayNextVO))))

(event Custom|TerminalTutorial
  (Default|TriggerMarker (Variables|Default|GetMarkerTerminal))
  (CallFunction|QueueVO "/Game/Audio/VoiceLines/Wav/WakeUp13.WakeUp13")
  (CallFunction|QueueVO "/Game/Audio/VoiceLines/Wav/WakeUp14.WakeUp14")
  (CallFunction|QueueVO "/Game/Audio/VoiceLines/Wav/WakeUp14_1.WakeUp14_1")
  (CallFunction|QueueVO "/Game/Audio/VoiceLines/Wav/WakeUp_15_1.WakeUp_15_1")
  (CallFunction|QueueVO "/Game/Audio/VoiceLines/Wav/WakeUp_15_2.WakeUp_15_2")
  (CallFunction|QueueVO "/Game/Audio/VoiceLines/Wav/WakeUp16.WakeUp16")
  (CallFunction|QueueVO "/Game/Audio/VoiceLines/Wav/WakeUp17.WakeUp17")
  (CallFunction|QueueVO "/Game/Audio/VoiceLines/Wav/WakeUp_Logs.WakeUp_Logs")
  (CallFunction|QueueVO "/Game/Audio/VoiceLines/Wav/WakeUp_Status.WakeUp_Status")
  (CallFunction|QueueVO "/Game/Audio/VoiceLines/Wav/WakeUp18.WakeUp18")
  (CallFunction|QueueVO "/Game/Audio/VoiceLines/Wav/WakeUp19.WakeUp19")
  (CallFunction|QueueVO "/Game/Audio/VoiceLines/Wav/WakeUp20.WakeUp20")
  (CallFunction|QueueVO "/Game/Audio/VoiceLines/Wav/WakeUp21.WakeUp21")
  (CallFunction|QueueVO "/Game/Audio/VoiceLines/Wav/WakeUp_21_1.WakeUp_21_1")
  (Math|Integer|IncrementInt (Variables|Default|GetCurrentStep)))

(event Custom|NoTutorial
  (bind _returnvalue (Game|GetPlayerCharacter 0))
  (Rendering|SetActorHiddenInGame _returnvalue false)
  (bind _aswbp_planet_choices (Utilities|Casting|CastToWBP_PlanetChoices (UserInterface|GetUserWidgetObject (Variables|/Game/Blueprints/BP_Terminal.BP_Terminal_C|GetPlanetChoices_WidgetScreen (Variables|Default|GetTerminalRef)))))
  (Default|StartRun _aswbp_planet_choices)
  (bind _asbp_first_person_character (Utilities|Casting|CastToBP_FirstPersonCharacter _returnvalue))
  (Default|AddVitalsUI _asbp_first_person_character)
  (Variables|Default|SetbTutorialOver true))

(event Custom|CheckForHint
  (bind _wbp_planetdetails_a_overlay (Variables|Default|GetWBP_PlanetDetails_A_Overlay))
  (bind _wbp_planetdetails_b_overlay (Variables|Default|GetWBP_PlanetDetails_B_Overlay))
  (bind _vo_counter (Variables|Default|GetVO_Counter))
  (bind _wbp_planetchoices_overlay (Variables|Default|GetWBP_PlanetChoices_Overlay))
  (bind _wbp_modules_overlay (Variables|Default|GetWBP_Modules_Overlay))
  (if (not (Variables|Default|GetbTutorialOver))
    (if (== _vo_counter 1)
      (Default|TriggerMarker (Variables|Default|GetMarkerTerminal))
      (elif (== _vo_counter 3)
        (Default|TriggerBox _wbp_planetdetails_a_overlay)
        (Default|TriggerBox _wbp_planetdetails_b_overlay)
        (elif (== _vo_counter 4)
          (Default|TriggerBox _wbp_planetdetails_a_overlay)
          (Default|TriggerBox _wbp_planetdetails_b_overlay)
          (Default|TriggerBoxDetails _wbp_planetdetails_a_overlay)
          (Default|TriggerBoxDetails _wbp_planetdetails_b_overlay)
          (elif (== _vo_counter 5)
            (Default|TriggerBoxButtonRight _wbp_planetchoices_overlay)
            (Default|TriggerBoxButtonLeft _wbp_planetchoices_overlay)
            (Default|TriggerBoxDetails _wbp_planetdetails_a_overlay)
            (Default|TriggerBoxDetails _wbp_planetdetails_b_overlay)
            (elif (== _vo_counter 6)
              (Default|TriggerBoxButtonRight _wbp_planetchoices_overlay)
              (Default|TriggerBoxButtonLeft _wbp_planetchoices_overlay)
              (Default|TriggerBoxButtonMiddle _wbp_planetchoices_overlay)
              (elif (== _vo_counter 7)
                (Default|TriggerBoxButtonMiddle _wbp_planetchoices_overlay)
                (elif (== _vo_counter 9)
                  (Default|TriggerBoxLogs _wbp_planetchoices_overlay)
                  (elif (== _vo_counter 10)
                    (Default|TriggerBoxLogs _wbp_planetchoices_overlay)
                    (Default|TriggerBoxStatus _wbp_planetchoices_overlay)
                    (elif (== _vo_counter 11)
                      (Default|TriggerBoxStatus _wbp_planetchoices_overlay)
                      (Default|TriggerBoxScout _wbp_planetdetails_a_overlay)
                      (Default|TriggerBoxScout _wbp_planetdetails_b_overlay)
                      (elif (== _vo_counter 12)
                        (Default|TriggerBoxScout _wbp_planetdetails_a_overlay)
                        (Default|TriggerBoxScout _wbp_planetdetails_b_overlay)
                        (Default|TriggerBox _wbp_modules_overlay)
                        (elif (== _vo_counter 13)
                          (Default|TriggerBox _wbp_modules_overlay)
                          (elif (== _vo_counter 14)
                            (bind _asbp_first_person_character (Utilities|Casting|CastToBP_FirstPersonCharacter (Game|GetPlayerCharacter 0)))
                            (Default|AddVitalsUI _asbp_first_person_character)
                            (elif (== _vo_counter 15)
                              (Default|TriggerMarker (Variables|Default|GetMarkerShelf))
                              (elif (== _vo_counter 17)
                                (Variables|Default|SetbTutorialOver true)))))))))))))))))

(event Custom|ShelfTutorial
  (Default|TriggerMarker (Variables|Default|GetMarkerShelf))
  (CallFunction|QueueVO "/Game/Audio/VoiceLines/Wav/WakeUp22.WakeUp22")
  (CallFunction|QueueVO "/Game/Audio/VoiceLines/Wav/WakeUp23.WakeUp23")
  (CallFunction|QueueVO "/Game/Audio/VoiceLines/Wav/WakeUp24.WakeUp24")
  (Math|Integer|IncrementInt (Variables|Default|GetCurrentStep)))

(event Custom|BeginTutorial
  (EventDispatchers|BindEventtoOnAudioFinished (Variables|Default|GetVO_Audio) (delegate Custom|OnVOFinished))
  (if (Variables|Default|GetbPlayIntro)
    (Default|BeginAlarm (Variables|Default|GetAlarmRef))
    (Rendering|SetActorHiddenInGame (Game|GetPlayerCharacter 0) true)
    (Transformation|SetWorldScale3D (Variables|/Script/Engine.StaticMeshActor|GetStaticMeshComponent (Variables|Default|GetEnergyTankRef)) (Math|Vector|MakeVector 0.0 0.0 0.0))
    (Rendering|SetVisibility (Variables|/Script/Engine.StaticMeshActor|GetStaticMeshComponent (Variables|Default|GetTerminalRef)) false true)
    (Rendering|SetVisibility (Variables|/Script/Engine.Light|GetLightComponent (Variables|Default|GetLight1Ref)) false false)
    (Rendering|SetVisibility (Variables|/Script/Engine.Light|GetLightComponent (Variables|Default|GetLight2Ref)) false false)
    (bind _returnvalue (Sequencer|Player|CreateLevelSequencePlayer (Variables|Default|GetIntroSequence)))
    (bind _output_get (Variables|Default|SetLSPlayer _returnvalue))
    (EventDispatchers|BindEventtoOnFinished _output_get (delegate Custom|Next%20steps))
    (Sequencer|Player|Play _output_get :!class /Script/MovieScene.MovieSceneSequencePlayer)
    (else
      (CallFunction|LightUp)
      (if (Variables|Default|GetbPlayTutorial)
        (CallFunction|NextSteps)
        (else
          (CallFunction|NoTutorial))))))

(event EventBeginPlay)

(event Collision|EventActorBeginOverlap
  (params (OtherActor :type Actor%20Object%20Reference)))

(event EventTick
  (params (DeltaSeconds :type Float%20%28single-precision%29)))

(fn ConstructionScript)

(fn QueueVO
  (params (Line :type Sound%20Wave%20Object%20Reference))
  (Utilities|Array|Add (Variables|Default|GetVOQueue) Line)
  (if (not (Variables|Default|GetbVOPlaying))
    (Development|PrintText "Calling play NextVO")
    (CallFunction|PlayNextVO)))

(fn PlayNextVO
  (bind _voqueue (Variables|Default|GetVOQueue))
  (bind _vo_audio (Variables|Default|GetVO_Audio))
  (if (== (Utilities|Array|Length _voqueue) 0)
    (Variables|Default|SetbVOPlaying false)
    (else
      (Variables|Default|SetbVOPlaying true)
      (bind _output_get (Variables|Default|SetLine (Utilities|Array|Get(acopy) _voqueue)))
      (Utilities|Array|RemoveIndex _voqueue)
      (Audio|Components|Audio|SetSound _vo_audio _output_get)
      (Audio|Components|Audio|Play _vo_audio 0.0))))

(fn LightUp
  (bind _alarmref (Variables|Default|GetAlarmRef))
  (Audio|Components|Audio|FadeOut (Variables|/Game/Blueprints/BP_Alarm.BP_Alarm_C|GetAlarmSound _alarmref) 3.0 0.0 "Linear" :!class /Script/Engine.AudioComponent)
  (Rendering|SetVisibility (Variables|/Game/Blueprints/BP_Alarm.BP_Alarm_C|GetSpotLight _alarmref) false false)
  (Rendering|SetVisibility (Variables|/Game/Blueprints/BP_Alarm.BP_Alarm_C|GetSpotLight1 _alarmref) false false)
  (Rendering|SetVisibility (Variables|/Script/Engine.StaticMeshActor|GetStaticMeshComponent (Variables|Default|GetTerminalRef)) true true)
  (Rendering|SetVisibility (Variables|/Script/Engine.Light|GetLightComponent (Variables|Default|GetLight1Ref)) true false)
  (Rendering|SetVisibility (Variables|/Script/Engine.Light|GetLightComponent (Variables|Default|GetLight2Ref)) true false))

(fn Tankon
  (Transformation|SetWorldScale3D (Variables|/Script/Engine.StaticMeshActor|GetStaticMeshComponent (Variables|Default|GetEnergyTankRef)) (Math|Vector|MakeVector 1.0 1.0 1.0)))

(fn NotifyTerminalOverlap
  (params (bPlayerInside :type Boolean))
  (Variables|Default|SetbTerminalPlayerInside bPlayerInside)
  (CallFunction|TryAdvancetoTerminal))

(fn TryAdvancetoTerminal
  (if (== (Variables|Default|GetCurrentStep) 1)
    (if (Variables|Default|GetbTerminalPlayerInside)
      (if (not (Variables|Default|GetbVOPlaying))
        (CallFunction|TerminalTutorial)))))

(fn NotifyShelfOverlap
  (params (bPlayerInside :type Boolean))
  (Variables|Default|SetbShelfPlayerInside bPlayerInside)
  (CallFunction|TryAdvancetoShelf))

(fn TryAdvancetoShelf
  (if (== (Variables|Default|GetCurrentStep) 2)
    (if (Variables|Default|GetbShelfPlayerInside)
      (if (not (Variables|Default|GetbVOPlaying))
        (CallFunction|ShelfTutorial)))))