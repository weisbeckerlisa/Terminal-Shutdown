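; BP_Button is an interactable toggle button that switches a tagged ship module on or off.
; On Interact, it flips its state and passes it with its ModuleTag to the ShipStateComponent on the player pawn.
; A dynamic material's emissive strength and an up or down tone at the button signal the new state.
; Buttons tagged Module.Shield also show or hide the referenced shield mesh directly.
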(event EventBeginPlay
  (bind _returnvalue (Rendering|Material|CreateDynamicMaterialInstance (Variables|Debug|GetStaticMeshComponent) 0 0 "None" :!class /Script/Engine.PrimitiveComponent))
  (bind _output_get (Variables|Default|SetButtonMID _returnvalue))
  (Rendering|Material|SetScalarParameterValue _output_get "EmissiveStrength" 0.0 :!class /Script/Engine.MaterialInstanceDynamic))

(event Collision|EventActorBeginOverlap
  (params (OtherActor :type Actor%20Object%20Reference)))

(event EventTick
  (params (DeltaSeconds :type Float%20%28single-precision%29)))

(event EventInteract
  (params (Hit :type Hit%20Result%20Structure))
  (bind _returnvalue (Game|Player|GetPlayerPawn 0))
  (bind _staticmeshcomponent (Variables|Debug|GetStaticMeshComponent))
  (bind _moduletag (Variables|Default|GetModuleTag))
  (bind _returnvalue_2 (Actor|GetComponentbyClass _returnvalue "/Script/TerminalShutdown.ShipStateComponent"))
  (bind _returnvalue_3 (Transformation|GetWorldLocation _staticmeshcomponent))
  (Utilities|IsValid _returnvalue_2
    (:Is%20Valid
      (bind _output_get (Variables|Default|SetbIsOn (not (Variables|Default|GetbIsOn))))
      (Class|ShipStateComponent|SetModuleEnabled _returnvalue_2 _moduletag _output_get)
      (if (Variables|Default|GetbIsOn)
        (Rendering|Material|SetScalarParameterValue (stale EventBeginPlay _output_get) "EmissiveStrength" 1.0 :!class /Script/Engine.MaterialInstanceDynamic)
        (Audio|PlaySoundatLocation "/Game/Audio/SciFiUISFX/Cues/Tone1/Octave/Tone1C_OctaveUp_Cue.Tone1C_OctaveUp_Cue" _returnvalue_3 "0, 0, 0" 1.0 1.0 0.0 0 0 0 0)
        (else
          (Rendering|Material|SetScalarParameterValue (stale EventBeginPlay _output_get) "EmissiveStrength" 0.0 :!class /Script/Engine.MaterialInstanceDynamic)
          (Audio|PlaySoundatLocation "/Game/Audio/SciFiUISFX/Cues/Tone1/Octave/Tone1D_OctaveDown_Cue.Tone1D_OctaveDown_Cue" _returnvalue_3 "0, 0, 0" 1.0 1.0 0.0 0 0 0 0)))
      (if (GameplayTags|MatchesTag "(TagName=\"Module.Shield\")" _moduletag)
        (Rendering|SetVisibility (Variables|/Script/Engine.StaticMeshActor|GetStaticMeshComponent (Variables|Default|GetShieldRef)) (Variables|Default|GetbIsOn) false)))))

(fn ConstructionScript)