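; BP_Fire is an extinguishable fire for a minigame, made of a Niagara effect and a point light, starting inactive and hidden.
; ApplyFireScale activates the effect and light and stores the fire's size.
; ApplyExtinguish shrinks the effect by strength, rate and delta time, hiding it at zero and notifying MiniGameController, without clearing IsActive.
; A collision sphere tracks whether a BP_FireExtinguisher is in range.
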(event OnComponentBeginOverlap(SphereCollision)
  (params (OverlappedComponent :type Primitive%20Component%20Object%20Reference) (OtherActor :type Actor%20Object%20Reference) (OtherComp :type Primitive%20Component%20Object%20Reference) (OtherBodyIndex :type Integer) (bFromSweep :type Boolean) (SweepResult :type Hit%20Result%20Structure%20%28by%20ref%29))
  (Utilities|Casting|CastToBP_FireExtinguisher OtherActor)
  (Variables|Default|SetbPlayerInRange true)
  (Development|PrintString "In range"))

(event OnComponentEndOverlap(SphereCollision)
  (params (OverlappedComponent :type Primitive%20Component%20Object%20Reference) (OtherActor :type Actor%20Object%20Reference) (OtherComp :type Primitive%20Component%20Object%20Reference) (OtherBodyIndex :type Integer))
  (Utilities|Casting|CastToBP_FireExtinguisher OtherActor)
  (Variables|Default|SetbPlayerInRange false)
  (Development|PrintString "Out of range"))

(event EventBeginPlay
  (bind _output_get (Variables|Default|SetbIsActive false))
  (Components|Activation|Deactivate (Variables|NiagaraActor|GetNiagaraComponent))
  (Variables|Default|SetFireScale 0.0)
  (Rendering|SetVisibility (Variables|Default|GetFire_PLight_BP) _output_get false))

(event EventTick
  (params (DeltaSeconds :type Float%20%28single-precision%29)))

(fn ConstructionScript)

(fn ApplyExtinguish
  (params (DeltaSeconds :type Float%20%28double-precision%29) (Strength :type Float%20%28double-precision%29))
  (bind _niagaracomponent (Variables|NiagaraActor|GetNiagaraComponent))
  (if (Variables|Default|GetbIsActive)
    (bind _output_get (Variables|Default|SetFireScale (Math|Float|Max(Float) 0.0 (- (Variables|Default|GetFireScale) (* DeltaSeconds Strength (Variables|Default|GetExtinguishRate))))))
    (Transformation|SetWorldScale3D _niagaracomponent (Math|Vector|MakeVector _output_get _output_get _output_get))
    (if (<= (Variables|Default|GetFireScale) 0.0)
      (Components|Activation|Deactivate _niagaracomponent)
      (Rendering|SetVisibility _niagaracomponent false true)
      (Rendering|SetVisibility (Variables|Default|GetFire_PLight_BP) false false)
      (Default|NotifyFireState (Variables|Default|GetMiniGameController)))))

(fn ApplyFireScale
  (params (FireScale :type Float%20%28double-precision%29))
  (bind _niagaracomponent (Variables|NiagaraActor|GetNiagaraComponent))
  (bind _output_get (Variables|Default|SetbIsActive true))
  (Rendering|SetVisibility _niagaracomponent _output_get true)
  (Components|Activation|Activate _niagaracomponent false)
  (Variables|Default|SetFireScale FireScale)
  (Rendering|SetVisibility (Variables|Default|GetFire_PLight_BP) true false))