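; BP_GOManager is the game-over manager that stages the ship game's victory and failure endings.
; PlayEndingSequence picks a level sequence by end reason, with starvation and dehydration sharing one, hides the player, plays it and calls the controller's EndScreen when finished.
; Separate events switch off ship lights and the terminal, trigger indexed Niagara effects, fade alarm and ambient audio, and swap planets for Earth.
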(event Custom|TurnOff
  (params (Index :type Integer))
  (bind _shiplight2 (Variables|Default|GetShipLight2))
  (bind _shiplight1 (Variables|Default|GetShipLight1))
  (bind _shiplight3 (Variables|Default|GetShipLight3))
  (bind _pointlightcomponent (Variables|/Script/Engine.PointLight|GetPointLightComponent _shiplight2))
  (bind _pointlightcomponent_2 (Variables|/Script/Engine.PointLight|GetPointLightComponent _shiplight1))
  (bind _pointlightcomponent_3 (Variables|/Script/Engine.PointLight|GetPointLightComponent _shiplight3))
  (switch int Index
    (:0
      (Rendering|Components|Light|SetIntensity _pointlightcomponent 0.0)
      (Rendering|SetVisibility _pointlightcomponent false true))
    (:1
      (Rendering|Components|Light|SetIntensity _pointlightcomponent_2 0.0)
      (Rendering|SetVisibility _pointlightcomponent_2 false true))
    (:2
      (Rendering|Components|Light|SetIntensity _pointlightcomponent_3 0.0)
      (Rendering|SetVisibility _pointlightcomponent_3 false true))
    (:3
      (Rendering|SetVisibility (Variables|/Script/Engine.StaticMeshActor|GetStaticMeshComponent (Variables|Default|GetTerminal)) false true))))

(event Custom|StartShutdownSound
  (bind _bgaudio (Variables|Default|GetBGAudio))
  (Audio|Components|Audio|SetSound _bgaudio "/Game/Audio/ShutDown.ShutDown")
  (Audio|Components|Audio|FadeIn _bgaudio 4.0 1.0 0.0 "Linear" :!class /Script/Engine.AudioComponent))

(event Custom|PlayEndingSequence
  (params (EndReason :type EEndReason%20Enum :default "None"))
  (switch Utilities|FlowControl|Switch|SwitchonEEndReason EndReason
    (:Victory
      (Variables|Default|SetEndingSequence "/Game/Blueprints/LS_GO_Earth.LS_GO_Earth"))
    (:ShipDestroyed
      (Variables|Default|SetEndingSequence "/Game/Blueprints/LS_GO_Damage.LS_GO_Damage"))
    (:EnergyDepleted
      (Variables|Default|SetEndingSequence "/Game/Blueprints/LS_GO_Energy.LS_GO_Energy"))
    (:Starvation
      (Variables|Default|SetEndingSequence "/Game/Blueprints/LS_GO_FoodWater.LS_GO_FoodWater" :!label _label))
    (:Dehydration
      (goto _label)))
  (bind _returnvalue (Sequencer|Player|CreateLevelSequencePlayer (Variables|Default|GetEndingSequence)))
  (bind _output_get (Variables|Default|SetLSPlayer _returnvalue))
  (EventDispatchers|BindEventtoOnFinished _output_get (delegate Custom|EndingScreen))
  (Rendering|SetActorHiddenInGame (Game|GetPlayerCharacter 0) true)
  (Sequencer|Player|Play _output_get :!class /Script/MovieScene.MovieSceneSequencePlayer))

(event Custom|EndingScreen
  (bind _asbp_first_person_player_controller (Utilities|Casting|CastToBP_FirstPersonPlayerController (Game|GetPlayerController 0)))
  (Default|EndScreen _asbp_first_person_player_controller))

(event Custom|StartBreath
  (bind _bgaudio (Variables|Default|GetBGAudio))
  (Audio|Components|Audio|SetSound _bgaudio "/Game/Audio/LastBreath.LastBreath")
  (Audio|Components|Audio|FadeIn _bgaudio 4.0 1.0 0.0 "Linear" :!class /Script/Engine.AudioComponent))

(event Custom|PlayVFX
  (params (Index :type Integer))
  (bind _endingvfx (Variables|Default|GetEndingVFX))
  (bind _output (Utilities|Array|Get(acopy) _endingvfx Index))
  (bind _niagaracomponent (Variables|/Script/Niagara.NiagaraActor|GetNiagaraComponent _output))
  (Components|Activation|Activate _niagaracomponent false)
  (Development|PrintString (Utilities|String|ToString(Text) (Utilities|Text|FormatText "Playing event with index: {index}" Index)))
  (Development|PrintString (Utilities|GetDisplayName _niagaracomponent)))

(event Custom|StartAlarm
  (Default|BeginAlarm (Variables|Default|GetAlarmRef))
  (Audio|Components|Audio|FadeIn (Variables|Default|GetBGAudio) 4.0 1.0 0.0 "Linear" :!class /Script/Engine.AudioComponent))

(event Custom|StopSounds
  (Audio|Components|Audio|FadeOut (Variables|/Game/Blueprints/BP_Alarm.BP_Alarm_C|GetAlarmSound (Variables|Default|GetAlarmRef)) 4.0 0.0 "Linear" :!class /Script/Engine.AudioComponent)
  (Audio|Components|Audio|FadeOut (Variables|Default|GetBGAudio) 4.0 0.0 "Linear" :!class /Script/Engine.AudioComponent)
  (Audio|Components|Audio|FadeOut (Variables|Default|GetEarRingAudio) 4.0 0.0 "Linear" :!class /Script/Engine.AudioComponent))

(event Custom|StartRing
  (Audio|Components|Audio|FadeIn (Variables|Default|GetEarRingAudio) 4.0 1.0 0.0 "Linear" :!class /Script/Engine.AudioComponent))

(event Custom|ShowEarth
  (bind _bgaudio (Variables|Default|GetBGAudio))
  (Rendering|SetActorHiddenInGame (Variables|Default|GetPlanetARef) true)
  (Rendering|SetActorHiddenInGame (Variables|Default|GetPlanetBRef) true)
  (Rendering|SetActorHiddenInGame (Variables|Default|GetEarthRef) false)
  (Audio|Components|Audio|SetSound _bgaudio "/Game/AbsoluteSpaceAndSciFi_VoltzSupreme/Cues/Stars_-_C_-_Orchestra_Cue.Stars_-_C_-_Orchestra_Cue")
  (Audio|Components|Audio|FadeIn _bgaudio 8.0 1.0 0.0 "Linear" :!class /Script/Engine.AudioComponent))

(event EventBeginPlay)

(event Collision|EventActorBeginOverlap
  (params (OtherActor :type Actor%20Object%20Reference)))

(event EventTick
  (params (DeltaSeconds :type Float%20%28single-precision%29)))

(fn ConstructionScript)