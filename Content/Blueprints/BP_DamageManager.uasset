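; Damage manager actor that shows escalating visual damage on the ship as it takes hits.
; It hides three stage lists of decals, meshes and emitters on BeginPlay, then binds to the planet choices object's OnShipDamaged event when initialized.
; Each damage level from 1 to 3 reveals its stage actors, lowers the ship lights' color temperature and passes the stage to LightFlicker.
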(event Custom|HandleDamage
  (params (Damage :type Integer))
  (bind _shiplights (Variables|Default|GetShipLights))
  (switch int Damage
    (:1
      (CallFunction|ShowAll (Variables|Default|GetStage1Actors))
      (CallFunction|SetLightsTemp _shiplights 5.5e+03))
    (:2
      (CallFunction|ShowAll (Variables|Default|GetStage2Actors))
      (CallFunction|SetLightsTemp _shiplights 4.9e+03))
    (:3
      (CallFunction|ShowAll (Variables|Default|GetStage3Actors))
      (CallFunction|SetLightsTemp _shiplights 4.2e+03)))
  (Class|LightFlickerComponent|ApplyDamageStage (Variables|Default|GetLightFlicker) Damage))

(event Custom|InitPlanetChoices
  (params (planetChoices :type WBP%20Planet%20Choices%20Object%20Reference))
  (bind _output_get (Variables|Default|SetPlanetChoicesRef planetChoices))
  (Utilities|IsValid _output_get
    (:Is%20Valid
      (Development|PrintString "Init planet choices ok")
      (EventDispatchers|BindEventtoOnShipDamaged _output_get (delegate Custom|HandleDamage)))))

(event EventBeginPlay
  (CallFunction|HideAll (Variables|Default|GetStage1Actors))
  (CallFunction|HideAll (Variables|Default|GetStage2Actors))
  (CallFunction|HideAll (Variables|Default|GetStage3Actors)))

(event Collision|EventActorBeginOverlap
  (params (OtherActor :type Actor%20Object%20Reference)))

(event EventTick
  (params (DeltaSeconds :type Float%20%28single-precision%29)))

(fn ConstructionScript)

(fn HideAll
  (params (ActorsList :type Array%20of%20Actor%20Object%20References))
  (for _array_element ActorsList
    (bind _asdcc_decal (Utilities|Casting|CastToDCC_Decal _array_element)
      (:then
        (Rendering|SetActorHiddenInGame _asdcc_decal true))
      (:CastFailed
        (bind _asstatic_mesh_actor (Utilities|Casting|CastToStaticMeshActor _array_element)
          (:then
            (Rendering|SetActorHiddenInGame _asstatic_mesh_actor true))
          (:CastFailed
            (bind _asemitter (Utilities|Casting|CastToEmitter _array_element))
            (Components|Activation|Deactivate (Variables|/Script/Engine.Emitter|GetParticleSystemComponent _asemitter))
            (Rendering|SetActorHiddenInGame _asemitter true)))))))

(fn ShowAll
  (params (ActorsList :type Array%20of%20Actor%20Object%20References))
  (for _array_element ActorsList
    (bind _asdcc_decal (Utilities|Casting|CastToDCC_Decal _array_element)
      (:then
        (Rendering|SetActorHiddenInGame _asdcc_decal false))
      (:CastFailed
        (bind _asstatic_mesh_actor (Utilities|Casting|CastToStaticMeshActor _array_element)
          (:then
            (Rendering|SetActorHiddenInGame _asstatic_mesh_actor false))
          (:CastFailed
            (bind _asemitter (Utilities|Casting|CastToEmitter _array_element))
            (Rendering|SetActorHiddenInGame _asemitter false)
            (Components|Activation|Activate (Variables|/Script/Engine.Emitter|GetParticleSystemComponent _asemitter) false)))))))

(fn SetLightsTemp
  (params (ShipLights :type Array%20of%20Point%20Light%20Object%20References) (Temperature :type Float%20%28double-precision%29))
  (for _array_element ShipLights
    (Class|LightComponent|SetTemperature (Variables|/Script/Engine.PointLight|GetPointLightComponent _array_element) Temperature)))

(fn NewFunction)