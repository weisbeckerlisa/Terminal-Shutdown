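; Ship terminal actor that hosts three widget screens: one for planet choices and two (A and B) for planet details.
; BeginPlay passes the left and right planet targets to the choices screen, then initializes all three with the run subsystem, player's ShipStateComponent and tutorial manager.
; Event bindings link the screens: choices refresh both details' selected side, while details trigger energy updates on choices.
; Completed minigame results are logged to the choices screen.
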(event Custom|CustomEvent
  (Default|SetSelectedSide (stale EventBeginPlay _aswbp_planet_details_a))
  (Default|SetSelectedSide (stale EventBeginPlay _aswbp_planet_details_b)))

(event Custom|UpdateEnergyA
  (Default|UpdateEnergy (stale EventBeginPlay _aswbp_planet_choices)))

(event Custom|LogsOnMiniGameCompleted
  (params (OutLogs :type Array%20of%20Texts))
  (Default|LogMiniGameResults (stale EventBeginPlay _aswbp_planet_choices) OutLogs))

(event Custom|UpdateEnergyB
  (Default|UpdateEnergy (stale EventBeginPlay _aswbp_planet_choices)))

(event EventBeginPlay
  (bind _returnvalue (Game|Player|GetPlayerPawn 0))
  (bind _returnvalue_2 (Subsystems|GetEventRunSubsystem))
  (bind _planetdetails_widgetscreen_b (Variables|Default|GetPlanetDetails_WidgetScreen_B))
  (bind _tutorialmanagerref (Variables|Default|GetTutorialManagerRef))
  (bind _planetdetails_widgetscreen_a (Variables|Default|GetPlanetDetails_WidgetScreen_A))
  (bind _aswbp_planet_choices (Utilities|Casting|CastToWBP_PlanetChoices (UserInterface|GetUserWidgetObject (Variables|Components|GetPlanetChoices_WidgetScreen))))
  (Default|SetPlanetTarget _aswbp_planet_choices (Variables|Default|GetPlanetLeftRef) (Variables|Default|GetPlanetRightRef))
  (Utilities|IsValid _returnvalue
    (:Is%20Valid
      (bind _asbp_first_person_character (Utilities|Casting|CastToBP_FirstPersonCharacter _returnvalue))
      (Utilities|IsValid _returnvalue_2
        (:Is%20Valid
          (Utilities|IsValid (Actor|GetComponentbyClass _asbp_first_person_character "/Script/TerminalShutdown.ShipStateComponent")
            (:Is%20Valid
              (Default|InitState _aswbp_planet_choices _returnvalue_2 (Actor|GetComponentbyClass _asbp_first_person_character "/Script/TerminalShutdown.ShipStateComponent") (Variables|Components|GetPlanetChoices_WidgetScreen) (Variables|Default|GetEnergyLevelRef) _tutorialmanagerref)
              (bind _aswbp_planet_details_a (Utilities|Casting|CastToWBP_PlanetDetails_A (UserInterface|GetUserWidgetObject _planetdetails_widgetscreen_a)))
              (Default|InitState _aswbp_planet_details_a _returnvalue_2 (Actor|GetComponentbyClass _asbp_first_person_character "/Script/TerminalShutdown.ShipStateComponent") _planetdetails_widgetscreen_a _tutorialmanagerref)
              (bind _aswbp_planet_details_b (Utilities|Casting|CastToWBP_PlanetDetails_B (UserInterface|GetUserWidgetObject _planetdetails_widgetscreen_b)))
              (Default|InitState _aswbp_planet_details_b _returnvalue_2 (Actor|GetComponentbyClass _asbp_first_person_character "/Script/TerminalShutdown.ShipStateComponent") _planetdetails_widgetscreen_b _tutorialmanagerref)
              (EventDispatchers|BindEventtoUpdateDetails _aswbp_planet_choices (delegate Custom|CustomEvent))
              (EventDispatchers|BindEventtoOnMiniGameCompleted (Variables|Default|GetMiniGameRunner) (delegate Custom|LogsOnMiniGameCompleted))
              (EventDispatchers|BindEventtoUpdateEnergy _aswbp_planet_details_a (delegate Custom|UpdateEnergyA))
              (EventDispatchers|BindEventtoUpdateEnergy _aswbp_planet_details_b (delegate Custom|UpdateEnergyB)))))))))

(event Collision|EventActorBeginOverlap
  (params (OtherActor :type Actor%20Object%20Reference)))

(event EventTick
  (params (DeltaSeconds :type Float%20%28single-precision%29)))

(fn ConstructionScript)