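; LS_Intro is the intro level sequence, with event-track handlers that drive a wake-up audio and tutorial opening.
; Six sequence events each play a different WakeUp sound at the world origin.
; Two events bound to BP_TutorialManager call LightUp and TankOn on the tutorial manager to trigger those moments during the cinematic.
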(event Custom|SequenceEvent_3
  (Audio|PlaySoundatLocation "/Game/Audio/VoiceLines/Wav/WakeUp5.WakeUp5" "0, 0, 0" "0, 0, 0" 1.0 1.0 0.0 0 0 0 0))

(event Custom|SequenceEvent_4
  (Audio|PlaySoundatLocation "/Game/Audio/VoiceLines/Wav/WakeUp6.WakeUp6" "0, 0, 0" "0, 0, 0" 1.0 1.0 0.0 0 0 0 0))

(event Custom|BP_TutorialManager_Event_0
  (params (BP_TutorialManager :type BP%20Tutorial%20Manager%20Object%20Reference))
  (Default|Tankon BP_TutorialManager))

(event Custom|SequenceEvent_0
  (Audio|PlaySoundatLocation "/Game/Audio/VoiceLines/Wav/WakeUp.WakeUp" "0, 0, 0" "0, 0, 0" 1.0 1.0 0.0 0 0 0 0))

(event Custom|SequenceEvent
  (Audio|PlaySoundatLocation "/Game/Audio/VoiceLines/Wav/WakeUp2.WakeUp2" "0, 0, 0" "0, 0, 0" 1.0 1.0 0.0 0 0 0 0))

(event Custom|SequenceEvent_1
  (Audio|PlaySoundatLocation "/Game/Audio/VoiceLines/Wav/WakeUp3.WakeUp3" "0, 0, 0" "0, 0, 0" 1.0 1.0 0.0 0 0 0 0))

(event Custom|SequenceEvent_2
  (Audio|PlaySoundatLocation "/Game/Audio/VoiceLines/Wav/WakeUp4.WakeUp4" "0, 0, 0" "0, 0, 0" 1.0 1.0 0.0 0 0 0 0))

(event Custom|BP_TutorialManager_Event
  (params (BP_TutorialManager :type BP%20Tutorial%20Manager%20Object%20Reference))
  (Default|LightUp BP_TutorialManager))