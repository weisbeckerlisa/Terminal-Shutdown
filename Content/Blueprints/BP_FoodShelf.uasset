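; Supply shelf actor that displays the ship's food and water stock and lets the player consume either by interacting with its collision.
; On BeginPlay it gets the ShipStateComponent from the first-person character, binds to its supplies-changed event and calls UpdateShelf.
; UpdateShelf destroys the spawned meshes, then FillShelf adds one collision-free static mesh per unit in a grid under each origin.
; Interact consumes a fixed amount of food or water depending on the component hit.
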(event EventBeginPlay
  (bind _asbp_first_person_character (Utilities|Casting|CastToBP_FirstPersonCharacter (Game|Player|GetPlayerPawn 0)))
  (bind _output_get (Variables|Default|SetShipRef (Actor|GetComponentbyClass _asbp_first_person_character "/Script/TerminalShutdown.ShipStateComponent")))
  (EventDispatchers|BindEventtoOnSuppliesChanged _output_get (EventDispatchers|CreateEvent :!event UpdateShelf))
  (CallFunction|UpdateShelf))

(event Collision|EventActorBeginOverlap
  (params (OtherActor :type Actor%20Object%20Reference)))

(event EventTick
  (params (DeltaSeconds :type Float%20%28single-precision%29)))

(event EventInteract
  (params (Hit :type Hit%20Result%20Structure))
  (bind _hitcomponent (Collision|BreakHitResult Hit))
  (bind _shipref (Variables|Default|GetShipRef))
  (if (== _hitcomponent (Variables|Default|GetFoodCollision))
    (Class|ShipStateComponent|ConsumeFood _shipref 2e+01)
    (elif (== _hitcomponent (Variables|Default|GetWaterCollision))
      (Class|ShipStateComponent|ConsumeWater _shipref 4e+01))))

(fn ConstructionScript)

(fn UpdateShelf
  (bind _spawnedfood (Variables|Default|GetSpawnedFood))
  (bind _spawnedwater (Variables|Default|GetSpawnedWater))
  (bind _shipref (Variables|Default|GetShipRef))
  (for _array_element _spawnedfood
    (Utilities|IsValid _array_element
      (:Is%20Valid
        (Components|DestroyComponent _array_element))))
  (Utilities|Array|Clear _spawnedfood)
  (for _array_element_2 _spawnedwater
    (Utilities|IsValid _array_element_2
      (:Is%20Valid
        (Components|DestroyComponent _array_element_2))))
  (Utilities|Array|Clear _spawnedwater)
  (CallFunction|FillShelf (Variables|Default|GetFoodOrigin) (Variables|Default|GetFoodMesh) (Variables|/Script/TerminalShutdown.ShipStateComponent|GetFoodUnits _shipref) (Variables|Default|GetSpawnedFood))
  (CallFunction|FillShelf (Variables|Default|GetWaterOrigin) (Variables|Default|GetWaterMesh) (Variables|/Script/TerminalShutdown.ShipStateComponent|GetWaterUnits _shipref) (Variables|Default|GetSpawnedWater)))

(fn FillShelf
  (params (Origin :type Scene%20Component%20Object%20Reference) (Mesh :type Static%20Mesh%20Object%20Reference) (Units :type Integer) (Array :type Array%20of%20Static%20Mesh%20Component%20Object%20References))
  (bind _columns (Variables|Default|GetColumns))
  (for _index (range 0 (- Units 1))
    (bind _output_get (Variables|Default|SetCurrRow (/ _index _columns)))
    (bind _output_get_2 (Variables|Default|SetCurrCol (Math|Integer|%(Integer) _index _columns)))
    (bind _returnvalue (AddComponent|AddStaticMeshComponent false))
    (Transformation|AttachComponentToComponent _returnvalue Origin "None" "KeepRelative" "KeepRelative" "KeepRelative" true)
    (Components|StaticMesh|SetStaticMesh _returnvalue Mesh)
    (Transformation|SetRelativeLocation _returnvalue (Math|Vector|MakeVector 0.0 (* _output_get_2 (Variables|Default|GetSpacingX)) (* _output_get (Variables|Default|GetSpacingY))) false false)
    (Collision|SetCollisionEnabled _returnvalue "NoCollision")
    (Utilities|Array|Add Array _returnvalue)))