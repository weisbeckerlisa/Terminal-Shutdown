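; BP_Pistol is a pistol the player picks up or drops through its Interact event, which toggles IsHeld.
; Pickup disables mesh physics and collision, snaps it to PistolSocket on the first-person mesh and clears its overlay material.
; Dropping detaches it in place and re-enables collision and physics.
; Both paths update IsHoldingPistol on the character and reuse the crosshair UI's ExtinguisherHeld flag.
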(event EventBeginPlay)

(event Collision|EventActorBeginOverlap
  (params (OtherActor :type Actor%20Object%20Reference)))

(event EventInteract
  (params (Hit :type Hit%20Result%20Structure))
  (bind _pistolmesh (Variables|Default|GetPistolMesh))
  (bind _asbp_first_person_character (Utilities|Casting|CastToBP_FirstPersonCharacter (Game|GetPlayerCharacter 0)))
  (if (Variables|Default|GetbIsHeld)
    (bind _output_get (Variables|Default|SetbIsHeld false))
    (bind _output_get_2 (Variables|/Game/UI/UI_Crosshair.UI_Crosshair_C|SetbExtinguisherHeld (Variables|/Game/FirstPerson/Blueprints/BP_FirstPersonCharacter.BP_FirstPersonCharacter_C|GetUI_CrosshairRef _asbp_first_person_character) _output_get))
    (Variables|/Game/FirstPerson/Blueprints/BP_FirstPersonCharacter.BP_FirstPersonCharacter_C|SetbIsHoldingPistol _asbp_first_person_character _output_get_2)
    (Transformation|DetachFromActor "KeepWorld" "KeepWorld" "KeepWorld")
    (Collision|SetCollisionEnabled _pistolmesh "QueryAndPhysics")
    (Physics|SetSimulatePhysics _pistolmesh true)
    (else
      (bind _output_get_3 (Variables|Default|SetbIsHeld true))
      (bind _output_get_4 (Variables|/Game/UI/UI_Crosshair.UI_Crosshair_C|SetbExtinguisherHeld (Variables|/Game/FirstPerson/Blueprints/BP_FirstPersonCharacter.BP_FirstPersonCharacter_C|GetUI_CrosshairRef _asbp_first_person_character) _output_get_3))
      (Variables|/Game/FirstPerson/Blueprints/BP_FirstPersonCharacter.BP_FirstPersonCharacter_C|SetbIsHoldingPistol _asbp_first_person_character _output_get_4)
      (Physics|SetSimulatePhysics _pistolmesh false)
      (Collision|SetCollisionEnabled _pistolmesh "NoCollision")
      (Transformation|ResetRelativeTransform _pistolmesh)
      (Transformation|AttachComponentToComponent (Variables|/Script/TerminalShutdown.TerminalShutdownCharacter|GetFirstPersonMesh _asbp_first_person_character) "PistolSocket" "SnapToTarget" "SnapToTarget" "SnapToTarget" false)
      (Rendering|Material|SetOverlayMaterial _pistolmesh 0 :!class /Script/Engine.MeshComponent))))

(fn ConstructionScript)