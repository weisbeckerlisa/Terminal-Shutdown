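; BP_FireExtinguisher is an interactable fire extinguisher that the player can pick up and drop.
; Interact toggles IsHeld: pickup disables physics and collision and attaches to a socket on player 0's character mesh, while drop detaches and restores both.
; When held, the static mesh takes the inverse of GripPivot's relative transform to align the grip with the socket.
; No spraying logic is present, and debug strings print on each toggle.
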(event EventBeginPlay)

(event Collision|EventActorBeginOverlap
  (params (OtherActor :type Actor%20Object%20Reference)))

(event EventTick
  (params (DeltaSeconds :type Float%20%28single-precision%29)))

(event EventInteract
  (params (Hit :type Hit%20Result%20Structure))
  (bind _staticmesh (Variables|Default|GetStaticMesh))
  (if (Variables|Default|GetbIsHeld)
    (Variables|Default|SetbIsHeld false)
    (Development|PrintString "Held off")
    (Transformation|DetachFromActor "KeepWorld" "KeepWorld" "KeepWorld")
    (Collision|SetCollisionEnabled _staticmesh "QueryAndPhysics")
    (Physics|SetSimulatePhysics _staticmesh true)
    (else
      (Variables|Default|SetbIsHeld true)
      (Development|PrintString "Held on")
      (Physics|SetSimulatePhysics _staticmesh false)
      (Collision|SetCollisionEnabled _staticmesh "NoCollision")
      (Transformation|AttachComponentToComponent (Variables|/Script/Engine.Character|GetMesh (Game|GetPlayerCharacter 0)) (Variables|Default|GetHoldSocketName) "SnapToTarget" "SnapToTarget" "KeepRelative" false)
      (Transformation|SetRelativeTransform _staticmesh (Math|Transform|InvertTransform (Transformation|GetRelativeTransform (Variables|Default|GetGripPivot))) false false))))

(fn ConstructionScript)