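; BP_Switch is an interactable switch that toggles a referenced light and can feed a mini-game.
; Interact flips IsOff, sets the light's root component visibility to match, and plays a click sound at the light's location rather than the switch's.
; If a MiniGameController is valid, the switch reports its Index and new state to it.
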(event EventBeginPlay)

(event Collision|EventActorBeginOverlap
  (params (OtherActor :type Actor%20Object%20Reference)))

(event EventTick
  (params (DeltaSeconds :type Float%20%28single-precision%29)))

(event EventInteract
  (params (Hit :type Hit%20Result%20Structure))
  (bind _lightref (Variables|Default|GetLightRef))
  (bind _minigamecontroller (Variables|Default|GetMiniGameController))
  (bind _rootcomponent (Variables|/Script/Engine.Actor|GetRootComponent _lightref))
  (bind _output_get (Variables|Default|SetbIsOff (not (Variables|Default|GetbIsOff))))
  (Rendering|SetVisibility _rootcomponent (not _output_get) false)
  (Audio|PlaySoundatLocation "/Game/Audio/SciFiUISFX/Cues/Clicks/Click_3_Cue.Click_3_Cue" (Transformation|GetWorldLocation _rootcomponent) "0, 0, 0" 1.0 1.0 0.0 0 0 0 0)
  (Utilities|IsValid _minigamecontroller
    (:Is%20Valid
      (Default|NotifySwitchState _minigamecontroller (Variables|Default|GetIndex) _output_get))))

(fn ConstructionScript)