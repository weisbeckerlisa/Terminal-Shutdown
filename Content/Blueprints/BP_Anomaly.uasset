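; BP_Anomaly is a hittable anomaly actor that turns to face the player camera every tick, billboard-style.
; When hit while active, HandeHit hides it, clears its active flag, notifies MGManager of the anomalies' state and spawns a particle effect at its location.
; The actor is only hidden, not destroyed, and nothing in this Blueprint reactivates it.
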(event EventBeginPlay)

(event Collision|EventActorBeginOverlap
  (params (OtherActor :type Actor%20Object%20Reference)))

(event EventTick
  (params (DeltaSeconds :type Float%20%28single-precision%29))
  (Transformation|SetActorRotation (Math|Rotator|FindLookatRotation (Transformation|GetActorLocation) (Camera|GetCameraLocation (Game|GetPlayerCameraManager 0)))))

(fn ConstructionScript)

(fn HandeHit
  (if (Variables|Default|GetbIsActive)
    (Rendering|SetActorHiddenInGame true)
    (Variables|Default|SetbIsActive false)
    (Default|NotifyAnomaliesState (Variables|Default|GetMG_Manager))
    (Effects|SpawnEmitteratLocation (Variables|Default|GetVFX) (Transformation|GetActorLocation))))