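; Level Sequence director for LS_GO_Damage, firing effect and sound events for what appears to be a damage sequence.
; Sequencer events call a bound BPGOManager to play VFX, start the alarm, start the ring and stop sounds.
; Each VFX event logs and passes a running index, then increments it, so successive triggers request successive effects.
; A separate unbound event plays a 2D explosion sound directly.
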(event Custom|BP_GOManager_Event
  (params (BP_GOManager :type BP%20GO%20Manager%20Object%20Reference))
  (bind _fvxindex (Variables|Default|GetFVXIndex))
  (Development|PrintString (Utilities|String|ToString(Text) (Utilities|Text|FormatText "calling event with index: {index}" _fvxindex)))
  (Default|PlayVFX BP_GOManager _fvxindex)
  (Math|Integer|IncrementInt _fvxindex))

(event Custom|SequenceEvent
  (Audio|PlaySound2D "/Game/Audio/Explosion.Explosion" 1.0 1.0 0.0 0 0))

(event Custom|BP_GOManager_Event_0
  (params (BP_GOManager :type BP%20GO%20Manager%20Object%20Reference))
  (Default|StartAlarm BP_GOManager))

(event Custom|BP_GOManager_Event_1
  (params (BP_GOManager :type BP%20GO%20Manager%20Object%20Reference))
  (Default|StartRing BP_GOManager))

(event Custom|BP_GOManager_Event_2
  (params (BP_GOManager :type BP%20GO%20Manager%20Object%20Reference))
  (Default|StopSounds BP_GOManager))